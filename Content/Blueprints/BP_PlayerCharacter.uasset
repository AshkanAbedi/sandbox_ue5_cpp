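; BP_PlayerCharacter is the player character Blueprint, whose graph holds hard-coded number-key bindings that exercise its InventoryComponent.
; Keys 1 to 3 add handgun ammo, a shotgun and the Black Room key from data assets, each printing an on-screen confirmation.
; Key 4 uses the item at index 0.
; BeginPlay, Tick, overlap and the construction script contain no logic.
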(event `Key|One`
  (params (Key :type "Key Structure"))
  (:`Pressed`
    (`InventoryComponent.AddItem` (`self.InventoryComponent`) "/Game/Blueprints/DA_Ammo_Handgun.DA_Ammo_Handgun" 5)
    (`KismetSystemLibrary.PrintString` "Ammo Added")))

(event `Key|Two`
  (params (Key :type "Key Structure"))
  (:`Pressed`
    (`InventoryComponent.AddItem` (`self.InventoryComponent`) "/Game/Blueprints/DA_Weaopn_Shotgun.DA_Weaopn_Shotgun" 1)
    (`KismetSystemLibrary.PrintString` "Shotgun Added")))

(event `Key|Three`
  (params (Key :type "Key Structure"))
  (:`Pressed`
    (`InventoryComponent.AddItem` (`self.InventoryComponent`) "/Game/Blueprints/DA_Key_BlackRoom.DA_Key_BlackRoom" 1)
    (`KismetSystemLibrary.PrintString` "Key Added")))

(event `Key|Four`
  (params (Key :type "Key Structure"))
  (:`Pressed`
    (`InventoryComponent.UseItem` (`self.InventoryComponent`) 0)))

(fn `UserConstructionScript`)